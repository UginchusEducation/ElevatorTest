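; Interaction component that detects BP_Interactible actors in front of the player's first-person camera.
; Every tick it runs a short object-type line trace from the camera, ignoring the player and drawing debug lines.
; A flag limits calls to transitions: gaining a hit stores the actor and calls CanInteractible, losing all hits calls FinishInteract.
; Switching directly between hit actors does not update the stored target.
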(event EventTick
  (params (DeltaSeconds :type Float%20%28single-precision%29))
  (bind _character (CallFunction|GetPlayerCharacterBP))
  (bind _firstpersoncamera (Variables|/Game/Blueprints/BP_FirstPersonCharacter.BP_FirstPersonCharacter_C|GetFirstPersonCamera _character))
  (bind _returnvalue (Transformation|GetWorldLocation _firstpersoncamera))
  (bind (_outhit _returnvalue_2) (Collision|LineTraceForObjects _returnvalue (+ _returnvalue (* (Math|Vector|GetForwardVector _firstpersoncamera) 125)) (Variables|Default|GetObject%20Types) false (Utilities|Array|MakeArray (CallFunction|GetPlayerCharacterBP)) "ForOneFrame"))
  (if _returnvalue_2
    (if (not (Variables|Default|GetbIsCanInteract))
      (Development|PrintString "Can Interact" true false "(R=0.342799,G=1.000000,B=0.087023,A=1.000000)" 5.0)
      (bind _asbp_interactible (Utilities|Casting|CastToBP_Interactible (.HitActor (Collision|BreakHitResult _outhit))))
      (Variables|Default|SetInteractibleActorRef _asbp_interactible)
      (Default|CanInteractible _asbp_interactible)
      (Variables|Default|SetbIsCanInteract true))
    (elif (Variables|Default|GetbIsCanInteract)
      (Development|PrintString "Interaction Finish" true false "(R=1.000000,G=0.089616,B=0.122781,A=1.000000)" 5.0)
      (Default|FinishInteract (Variables|Default|GetInteractibleActorRef))
      (Variables|Default|SetbIsCanInteract false))))