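; Interactable floor button for a building elevator that calls the elevator to its assigned floor when used.
; On interaction it sends GoToFloor to the building's elevator, then ends the interaction when the elevator reports it finished lifting to that floor.
; Timelines blend the button's color between idle, can-interact and interacted states through dynamic material instances created for button and backplate in the construction script.
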(event Custom|ElevatorEndLifting
  (params (LiftToFloor :type Integer))
  (if (== LiftToFloor (Variables|Building|GetFloorButton))
    (CallFunction|EndInteract)))

(event EventBeginPlay
  (EventDispatchers|BindEventtoOnElevatorFinishLift (Variables|/Game/Blueprints/Building/BP_Building.BP_Building_C|GetElevatorRef (Variables|Building|GetBuildingRef)) (delegate Custom|ElevatorEndLifting)))

(event EventCanInteractible
  (|CallParentFunction)
  ;[1 1 1] Can Interact Button Animation
  (bind _value (Timeline|ChangeButton Play)
    (:Update
      (Rendering|Material|SetVectorParameterValue (Variables|Default|GetButtonDynMat) "Color" (Math|Color|Lerp(LinearColor) (Variables|Color|GetButtonColor) (Variables|Color|GetCanInteractButtonColor) _value) :!class /Script/Engine.MaterialInstanceDynamic))))

(event EventFinishInteract
  (|CallParentFunction)
  ;[1 1 1] Can Interact Button Animation
  (bind _value (Timeline|ChangeButton Reverse)
    (:Update
      (Rendering|Material|SetVectorParameterValue (Variables|Default|GetButtonDynMat) "Color" (Math|Color|Lerp(LinearColor) (Variables|Color|GetButtonColor) (Variables|Color|GetCanInteractButtonColor) _value) :!class /Script/Engine.MaterialInstanceDynamic))))

(event EventStartInteract
  (|CallParentFunction)
  (Default|GotoFloor (Variables|/Game/Blueprints/Building/BP_Building.BP_Building_C|GetElevatorRef (Variables|Building|GetBuildingRef)) (Variables|Building|GetFloorButton))
  (bind _value (Timeline|Timeline Play)
    (:Update
      (Rendering|Material|SetVectorParameterValue (Variables|Default|GetButtonDynMat) "Color" (Math|Color|Lerp(LinearColor) (Variables|Color|GetCanInteractButtonColor) (Variables|Color|GetInteractedButtonColor) _value) :!class /Script/Engine.MaterialInstanceDynamic))))

(event EventEndInteract
  (|CallParentFunction)
  (bind _value (Timeline|Timeline Reverse)
    (:Update
      (Rendering|Material|SetVectorParameterValue (Variables|Default|GetButtonDynMat) "Color" (Math|Color|Lerp(LinearColor) (Variables|Color|GetCanInteractButtonColor) (Variables|Color|GetInteractedButtonColor) _value) :!class /Script/Engine.MaterialInstanceDynamic))))

(fn ConstructionScript
  (Utilities|FlowControl|Sequence
    (:then_0
      (bind _returnvalue (Rendering|Material|CreateDynamicMaterialInstance "/Game/Elevator/Materials/MI_BC_Button.MI_BC_Button" "None" "None" :!class /Script/Engine.KismetMaterialLibrary))
      (bind _output_get (Variables|Default|SetButtonDynMat _returnvalue))
      (Rendering|Material|SetMaterial (Variables|Default|GetButton) 0 _output_get)
      (Rendering|Material|SetVectorParameterValue (Variables|Default|GetButtonDynMat) "Color" (Variables|Color|GetButtonColor) :!class /Script/Engine.MaterialInstanceDynamic))
    (:then_1
      (bind _returnvalue_2 (Rendering|Material|CreateDynamicMaterialInstance "/Game/Elevator/Materials/MI_BC_Button.MI_BC_Button" "None" "None" :!class /Script/Engine.KismetMaterialLibrary))
      (bind _output_get_2 (Variables|Default|SetButtonBackDynMat _returnvalue_2))
      (Rendering|Material|SetMaterial (Variables|Default|GetButtonBack) 0 _output_get_2)
      (Rendering|Material|SetVectorParameterValue (Variables|Default|GetButtonBackDynMat) "Color" (Variables|Color|GetButtonBackColor) :!class /Script/Engine.MaterialInstanceDynamic))))