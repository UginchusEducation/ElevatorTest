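; Elevator actor that rides between a building's floor points, with a procedurally built cage and a per-floor button panel.
; The construction script stacks border and door bars, and BeginPlay snaps it to the current floor and spawns attached buttons in a grid.
; GoToFloor ignores requests while busy, otherwise scales the door bars shut and lerps transforms via a distance-scaled timeline.
; On arrival it calls an elevator-arrived event and reopens the door.
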(event Custom|GoToFloor
  (params (NextFloor :type Integer))
  ;[1 1 1] Prepare Elevator
  (if (Variables|Default|GetbCanLift)
    (Variables|Default|SetbCanLift false)
    (bind _output_get (Variables|Floor|SetNextFloor NextFloor))
    (Development|PrintString (Utilities|String|Append "[Elevator] Go to floor = " (Utilities|String|ToString(Integer) _output_get)) false true "(R=0.000000,G=0.660000,B=1.000000,A=1.000000)" 5.0)
    (CallFunction|CalculateFloorsDistance)
    (CallFunction|CloseElevatorDoor)
    (CallFunction|StartElevate)
    (else
      (Development|PrintString (Utilities|String|Append "[Elevator] Elevator is busy" "") false true "(R=0.000000,G=0.660000,B=1.000000,A=1.000000)" 5.0))))

(event Custom|StartElevate
  ;[1 1 1] Elevator Moving
  (bind _value (Timeline|ElevatorMoving PlayFromStart)
    (:Update
      (Transformation|SetActorTransform (Math|Transform|Lerp(Transform) (Variables|Default|GetCurrentFloorTransform) (Variables|Default|GetNextFloorTransform) _value)))
    (:Finished
      (Variables|Default|SetbCanLift true)
      (bind _output_get (Variables|Floor|SetCurrentFloor (Variables|Floor|GetNextFloor)))
      (Default|CallOnElevatorLifttotheFloor _output_get)
      (CallFunction|OpenElevatorDoor))))

(event Custom|CloseElevatorDoor
  ;[1 1 1] Open / Close Door
  (bind _newtrack_0 (Timeline|ElevatorDoor PlayFromStart)
    (:Update
      (for _array_element (Variables|Default|GetElevatorDoorArr)
        (Transformation|SetWorldScale3D _array_element (Math|Vector|MakeVector 0.1 (+ (* _newtrack_0 1.9) 0.1) 0.1))))))

(event Custom|OpenElevatorDoor
  ;[1 1 1] Open / Close Door
  (bind _newtrack_0 (Timeline|ElevatorDoor ReverseFromEnd)
    (:Update
      (for _array_element (Variables|Default|GetElevatorDoorArr)
        (Transformation|SetWorldScale3D _array_element (Math|Vector|MakeVector 0.1 (+ (* _newtrack_0 1.9) 0.1) 0.1))))))

(event EventBeginPlay
  (bind _buildingref (Variables|Default|GetBuildingRef))
  (CallFunction|SpawnElevatorButton)
  (Transformation|SetActorTransform (Transformation|GetWorldTransform (Utilities|Array|Get(acopy) (Variables|/Game/Blueprints/Building/BP_Building.BP_Building_C|GetFloorElevatorPoint _buildingref) (- (Variables|Floor|GetCurrentFloor) (Variables|/Game/Blueprints/Building/BP_Building.BP_Building_C|GetStartFloor _buildingref))))))

(fn ConstructionScript
  (Utilities|FlowControl|Sequence
    (:then_0
      (CallFunction|ClearAllGeneratedMesh))
    (:then_1
      (for _index (range 0 (- (LocalVariables|GetBorderLineCount) 1))
        (bind _output_get (LocalVariables|SetIndex _index))
        (LocalVariables|SetZHigh (Math|Conversions|ToFloat(Integer) (+ (* _output_get 50) 50)))
        (Utilities|FlowControl|Sequence
          (:then_0
            (bind _returnvalue (AddComponent|AddStaticMeshComponent false (Math|Transform|MakeTransform (Math|Vector|MakeVector 0.0 2e+02 (LocalVariables|GetZHigh)) "0, 0, 0" "0.100000,6.000000,0.100000")))
            (Utilities|Array|Add (Variables|Default|GetBorderArr) _returnvalue))
          (:then_1
            (bind _returnvalue_2 (AddComponent|AddStaticMeshComponent false (Math|Transform|MakeTransform (Math|Vector|MakeVector 0.0 0.0 (LocalVariables|GetZHigh)) "0, 0, 0" "3.000000,0.100000,0.100000")))
            (Utilities|Array|Add (Variables|Default|GetBorderArr) _returnvalue_2))
          (:then_2
            (bind _returnvalue_3 (AddComponent|AddStaticMeshComponent false (Math|Transform|MakeTransform (Math|Vector|MakeVector 2.9e+02 3e+02 (LocalVariables|GetZHigh)) "0, 0, 0" "0.100000,5.000000,0.100000")))
            (Utilities|Array|Add (Variables|Default|GetBorderArr) _returnvalue_3))
          (:then_3
            (bind _returnvalue_4 (AddComponent|AddStaticMeshComponent false (Math|Transform|MakeTransform (Math|Vector|MakeVector 0.0 7.9e+02 (LocalVariables|GetZHigh)) "0, 0, 0" "3.000000,0.100000,0.100000")))
            (Utilities|Array|Add (Variables|Default|GetBorderArr) _returnvalue_4))
          (:then_4
            (bind _returnvalue_5 (AddComponent|AddStaticMeshComponent false (Math|Transform|MakeTransform (Math|Vector|MakeVector 0.0 0.0 (LocalVariables|GetZHigh)) "0, 0, 0" "0.100000,0.100000,0.100000")))
            (Utilities|Array|Add (Variables|Default|GetElevatorDoorArr) _returnvalue_5)))))))

(fn CalculateFloorsDistance
  (Variables|Default|SetCurrentFloorTransform (Transformation|GetActorTransform))
  ;[1 1 1] Set Elevator Destination
  (Variables|Default|SetNextFloorTransform (Transformation|GetWorldTransform (Utilities|Array|Get(acopy) (Variables|/Game/Blueprints/Building/BP_Building.BP_Building_C|GetFloorElevatorPoint (Variables|Default|GetBuildingRef)) (- (Variables|Floor|GetNextFloor) (Variables|/Game/Blueprints/Building/BP_Building.BP_Building_C|GetStartFloor (Variables|Default|GetBuildingRef))))))
  ;[1 1 1] Set Elevator Speed
  (Components|Timeline|SetPlayRate (Variables|Default|GetElevatorMoving) (/ (Variables|Default|GetElevatorSpeed) (Math|Conversions|ToFloat(Integer) (Math|Integer|Absolute(Integer) (- (Variables|Floor|GetNextFloor) (Variables|Floor|GetCurrentFloor)))))))

(fn FinishElevate)

(fn SpawnElevatorButton
  (bind _returnvalue (Transformation|GetActorRotation))
  (bind _buildingref (Variables|Default|GetBuildingRef))
  (for _index (range 0 (- (Variables|/Game/Blueprints/Building/BP_Building.BP_Building_C|GetFloorCount _buildingref) (Variables|/Game/Blueprints/Building/BP_Building.BP_Building_C|GetStartFloor _buildingref)))
    (LocalVariables|SetIndex _index)
    (bind _returnvalue_2 (Game|SpawnActorfromClass "/Game/Blueprints/Interactible/BP_ElevatorButton.BP_ElevatorButton_C" (Math|Transform|MakeTransform (Math|Vector|MakeVector 2.9e+02 (+ (Math|Conversions|ToFloat(Integer) (* (/ (LocalVariables|GetIndex) (LocalVariables|GetFloorMaxAmount)) (LocalVariables|GetYDistanceButton))) 5e+01) (+ 1.2e+02 (* (Math|Integer|%(Integer) (LocalVariables|GetIndex) (LocalVariables|GetFloorMaxAmount)) 15) (.z (Transformation|GetActorLocation)))) (Math|Rotator|MakeRotator (.roll _returnvalue) (.pitch _returnvalue) (+ (.yaw _returnvalue) 9e+01)) "1.000000,1.000000,1.000000") "Undefined" "MultiplyWithRoot" 0 (+ (LocalVariables|GetIndex) (Variables|/Game/Blueprints/Building/BP_Building.BP_Building_C|GetStartFloor (Variables|Default|GetBuildingRef))) (Variables|Default|GetBuildingRef) 0))
    (Transformation|AttachActorToActor _returnvalue_2 self "None" "KeepRelative" "KeepRelative" "KeepRelative" true)))

(fn ClearAllGeneratedMesh
  (bind _elevatordoorarr (Variables|Default|GetElevatorDoorArr))
  (bind _borderarr (Variables|Default|GetBorderArr))
  (Utilities|FlowControl|Sequence
    (:then_0
      (for _array_element _borderarr
        (Components|DestroyComponent _array_element))
      (Utilities|Array|Clear _borderarr))
    (:then_1
      (for _array_element_2 _elevatordoorarr
        (Components|DestroyComponent _array_element_2))
      (Utilities|Array|Clear _elevatordoorarr))))