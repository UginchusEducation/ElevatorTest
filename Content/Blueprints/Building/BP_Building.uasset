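; Procedural multi-floor building actor with switchback stairs and an elevator.
; Construction script clears and rebuilds components for each floor from StartFloor to FloorCount: slabs, floor-number text, stairs between floors, and sphere markers for elevator stops and call buttons.
; BeginPlay spawns BP_Elevator, falling back to StartFloor if its starting floor is out of range, and a BP_BuildingElevatorButton at each button marker, passing both a building reference.
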(event EventBeginPlay
  (BlueprintSpawn|SpawnElevator)
  (BlueprintSpawn|SpawnBuildingElevatorButton))

(fn ConstructionScript
  (CallFunction|ClearAllPrevInstance)
  (for _index (range (- (Variables|BuildingSettings|Floor|GetStartFloor) 1) (- (Variables|BuildingSettings|Floor|GetFloorCount) 1))
    (bind _output_get (LocalVariables|SetFloorIndex _index))
    (LocalVariables|SetZFloorPosition (* _output_get (Variables|BuildingSettings|Floor|GetFloorHeight)))
    (Utilities|FlowControl|Sequence
      (:then_0
        (CallFunction|CreateFloor (LocalVariables|GetZFloorPosition) (LocalVariables|GetFloorIndex)))
      (:then_1
        ;[1 1 1] Final Floor Check
        (if (not (== (LocalVariables|GetFloorIndex) (- (Variables|BuildingSettings|Floor|GetFloorCount) 1)))
          (CallFunction|CreateStairs (LocalVariables|GetZFloorPosition)))))))

(fn CreateStairs
  (params (ZPosition :type Float%20%28double-precision%29))
  (Utilities|FlowControl|Sequence
    (:then_0
      ;[1 1 1] First floor platform
      (bind _returnvalue (AddComponent|AddStaticMeshComponent false (Math|Transform|MakeTransform (Math|Vector|MakeVector -2e+02 0.0 ZPosition) "0, 0, 0" "4.000000,2.000000,0.100000")))
      (Utilities|Array|Add (Variables|FloorComponent|GetFloorMeshArr) _returnvalue))
    (:then_1
      ;[1 1 1] First floor stairs
      (bind _returnvalue_2 (AddComponent|AddStaticMeshComponent false (Math|Transform|MakeTransform (Math|Vector|MakeVector 0.0 2e+02 ZPosition) "0.000000,0.000000,-25.000000" "2.000000,5.000000,0.100000")))
      (Utilities|Array|Add (Variables|FloorComponent|GetFloorMeshArr) _returnvalue_2))
    (:then_2
      ;[1 1 1] First to Second floor platform
      (bind _returnvalue_3 (AddComponent|AddStaticMeshComponent false (Math|Transform|MakeTransform (Math|Vector|MakeVector -2e+02 6.5e+02 (+ ZPosition (/ (Variables|BuildingSettings|Floor|GetFloorHeight) 2.0))) "0, 0, 0" "4.000000,2.000000,0.100000")))
      (Utilities|Array|Add (Variables|FloorComponent|GetFloorMeshArr) _returnvalue_3))
    (:then_3
      ;[1 1 1] Second floor stairs
      (bind _returnvalue_4 (AddComponent|AddStaticMeshComponent false (Math|Transform|MakeTransform (Math|Vector|MakeVector 0.0 6.5e+02 (+ ZPosition (/ (Variables|BuildingSettings|Floor|GetFloorHeight) 2.0))) "0.000000,180.000000,-25.000000" "2.000000,5.000000,0.100000")))
      (Utilities|Array|Add (Variables|FloorComponent|GetFloorMeshArr) _returnvalue_4))
    (:then_4
      ;[1 1 1] First floor platform
      (bind _returnvalue_5 (AddComponent|AddStaticMeshComponent false (Math|Transform|MakeTransform (Math|Vector|MakeVector -2e+02 0.0 (+ ZPosition (Variables|BuildingSettings|Floor|GetFloorHeight))) "0, 0, 0" "4.000000,2.000000,0.100000")))
      (Utilities|Array|Add (Variables|FloorComponent|GetFloorMeshArr) _returnvalue_5))))

(fn ClearAllPrevInstance
  (bind _floortextarr (Variables|FloorComponent|GetFloorTextArr))
  (bind _floormesharr (Variables|FloorComponent|GetFloorMeshArr))
  (bind _floorelevatorpoint (Variables|FloorComponent|GetFloorElevatorPoint))
  (bind _floorelevatorbutton (Variables|FloorComponent|GetFloorElevatorButton))
  (Utilities|FlowControl|Sequence
    (:then_0
      ;[1 1 1] Clear All Meshes
      (for _array_element _floormesharr
        (Components|DestroyComponent _array_element))
      (Utilities|Array|Clear _floormesharr))
    (:then_1
      ;[1 1 1] Clear All Text
      (for _array_element_2 _floortextarr
        (Components|DestroyComponent _array_element_2))
      (Utilities|Array|Clear _floortextarr))
    (:then_2
      ;[1 1 1] Clear All Points for Elevator
      (for _array_element_3 _floorelevatorpoint
        (Components|DestroyComponent _array_element_3))
      (Utilities|Array|Clear _floorelevatorpoint))
    (:then_3
      ;[1 1 1] Clear All Points for Floor Elevator Button
      (for _array_element_4 _floorelevatorbutton
        (Components|DestroyComponent _array_element_4))
      (Utilities|Array|Clear _floorelevatorbutton))))

(fn CreateFloor
  (params (ZPosition :type Float%20%28double-precision%29) (Index :type Integer))
  (Utilities|FlowControl|Sequence
    (:then_0
      ;[1 1 1] Floor big platform
      (bind _returnvalue (AddComponent|AddStaticMeshComponent false (Math|Transform|MakeTransform (Math|Vector|MakeVector 2e+02 0.0 ZPosition) "0, 0, 0" "8.000000,8.000000,0.100000")))
      (Utilities|Array|Add (Variables|FloorComponent|GetFloorMeshArr) _returnvalue)
      (bind _returnvalue_2 (AddComponent|AddStaticMeshComponent false (Math|Transform|MakeTransform (Math|Vector|MakeVector 9e+02 0.0 ZPosition) "0, 0, 0" "1.000000,0.100000,4.000000")))
      (Utilities|Array|Add (Variables|FloorComponent|GetFloorMeshArr) _returnvalue_2))
    (:then_1
      ;[1 1 1] Add Text
      (bind _returnvalue_3 (AddComponent|AddTextRenderComponent false (Math|Transform|MakeTransform (Math|Vector|MakeVector 9.5e+02 2e+01 (+ ZPosition 3.5e+02)) "0.000000,90.000000,0.000000" "1.000000,1.000000,1.000000")))
      (Rendering|Components|TextRender|SetText _returnvalue_3 (Utilities|Text|ToText(Integer) (+ 1 Index)))
      (Utilities|Array|Add (Variables|FloorComponent|GetFloorTextArr) _returnvalue_3)
      (bind _returnvalue_4 (AddComponent|AddTextRenderComponent false (Math|Transform|MakeTransform (Math|Vector|MakeVector 9.5e+02 -1e+01 (+ ZPosition 3.5e+02)) "0.000000,-90.000000,0.000000" "1.000000,1.000000,1.000000")))
      (Rendering|Components|TextRender|SetText _returnvalue_4 (Utilities|Text|ToText(Integer) (+ 1 Index)))
      (Utilities|Array|Add (Variables|FloorComponent|GetFloorTextArr) _returnvalue_4))
    (:then_2
      ;[1 1 1] Elevator Point
      (bind _returnvalue_5 (AddComponent|AddSphereComponent false (Math|Transform|MakeTransform (Math|Vector|MakeVector 1e+03 0.0 ZPosition) "0, 0, 0" "1.000000,1.000000,1.000000")))
      (Utilities|Array|Add (Variables|FloorComponent|GetFloorElevatorPoint) _returnvalue_5)
      (bind _returnvalue_6 (AddComponent|AddSphereComponent false (Math|Transform|MakeTransform (Math|Vector|MakeVector 9.5e+02 1e+01 (+ ZPosition 1.5e+02)) "0, 0, 0" "1.000000,1.000000,1.000000")))
      (Utilities|Array|Add (Variables|FloorComponent|GetFloorElevatorButton) _returnvalue_6))))

(fn SpawnElevator
  (Utilities|FlowControl|Sequence
    (:then_0
      ;[1 1 1] Elevator Location
      (if (or (< (Variables|BuildingSettings|Elevator|GetElevatorStartingFloor) (Variables|BuildingSettings|Floor|GetStartFloor)) (> (Variables|BuildingSettings|Elevator|GetElevatorStartingFloor) (Variables|BuildingSettings|Floor|GetFloorCount)))
        (Variables|BuildingSettings|Elevator|SetElevatorStartingFloor (Variables|BuildingSettings|Floor|GetStartFloor))
        (Development|PrintString (Utilities|String|Append "[Building] The building does not have a " (Utilities|String|ToString(Integer) (Variables|BuildingSettings|Elevator|GetElevatorStartingFloor)) "th floor, the elevator will be on the ground floor ") true true "(R=1.000000,G=0.161778,B=0.000000,A=1.000000)" 1e+01)))
    (:then_1
      (bind _returnvalue (Game|SpawnActorfromClass "/Game/Blueprints/Building/BP_Elevator.BP_Elevator_C" (Math|Transform|MakeTransform "0, 0, 0" "0, 0, 0" "1.000000,1.000000,1.000000") "Undefined" "MultiplyWithRoot" 0 self (Variables|BuildingSettings|Elevator|GetElevatorStartingFloor) (Variables|BuildingSettings|Elevator|GetElevator%20Speed) 0))
      (Variables|Elevator|SetElevatorRef _returnvalue))))

(fn SpawnBuildingElevatorButton
  (for (_array_element _array_index) (Variables|FloorComponent|GetFloorElevatorButton)
    (Game|SpawnActorfromClass "/Game/Blueprints/Interactible/BP_BuildingElevatorButton.BP_BuildingElevatorButton_C" (Transformation|GetWorldTransform _array_element) "Undefined" "MultiplyWithRoot" 0 (+ _array_index (Variables|BuildingSettings|Floor|GetStartFloor)) self 0)))